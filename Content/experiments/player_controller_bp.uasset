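; Experimental player controller that sets up the HUD, triggers vehicle spawning and manages switching between UI and game input.
; BeginPlay creates the controller widget and calls Spawn on every VehicleSpawnPoint in the level.
; Possessing a pawn passes it and the widget's spawn-unit button to SetUIForPawn.
; Space toggles the cursor, and two events set input modes, with SetUIOnly actually applying Game and UI.
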(event `self.ReceiveBeginPlay`
  ;[1 1 1] add UI to view
  (`KismetSystemLibrary.PrintString` "created UI widget")
  (bind _returnvalue (`|CreateWidget` "/Game/experiments/controller_ui_widget.controller_ui_widget_C" (`GameplayStatics.GetPlayerController` 0)))
  (`UserWidget.AddToViewport` _returnvalue 0)
  (bind _output_get (set `self.UIWidget` _returnvalue))
  ;[1 1 1] spawn vehicles from spawnpoints
  (bind _outactors (`GameplayStatics.GetAllActorsOfClass` "/Script/UA2.VehicleSpawnPoint"))
  (for _array_element _outactors
    (`VehicleSpawnPoint.Spawn` _array_element)))

(event `self.Set_UI_only`
  ;[1 1 1] switch between ui and game mode
  (`WidgetBlueprintLibrary.SetInputMode_GameAndUIEx` self null "DoNotLock" false))

(event `Key|SpaceBar`
  (params (Key :type "Key Structure"))
  ;[1 1 1] switch between ui and game mode
  (:`Pressed`
    (`self.ToggleMouseCursor`)))

(event `self.ReceivePossess`
  (params (PossessedPawn :type "Pawn Object Reference"))
  (bind _ascontroller_ui_widget (cast `/Game/experiments/controller_ui_widget` (stale `self.ReceiveBeginPlay` _output_get)))
  (`self.SetUIForPawn` PossessedPawn (`/Game/experiments/controller_ui_widget.SpawnUnitButton` _ascontroller_ui_widget)))

(event `self.Set_Game_only`
  ;[1 1 1] switch between ui and game mode
  (`WidgetBlueprintLibrary.SetInputMode_GameOnly` self))

(fn `UserConstructionScript`)
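; TankUnitBP is a player-controllable tank that drives on four child-actor wheels and has an aimable turret with switchable camera views.
; BeginPlay passes the wheels, turret base, barrel and first-person camera to FindComponents and registers the tank with its NavigationComponent.
; Look inputs aim the turret in first person or orbit the third-person camera, which also zooms.
; SetWidgetTeam applies the team to the world icon and adds the unit to the HUD.
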(event `InputAxis|forward`
  (params (AxisValue :type "Float (single-precision)"))
  ;[1 1 1] driving wheels
  (`self.ControlWheels` AxisValue (stale `InputAxis|turn_right` AxisValue)))

(event `InputAxis|turn_right`
  (params (AxisValue :type "Float (single-precision)"))
  ;[1 1 1] driving wheels
  (`self.ControlWheels` (stale `InputAxis|forward` AxisValue) AxisValue))

(event `InputAction|switch_view`
  (params (Key :type "Key Structure"))
  ;[1 1 1] camera controls
  (:`Pressed`
    (`self.SwitchCameraView`)))

(event `InputAxis|AimElevation`
  (params (AxisValue :type "Float (single-precision)"))
  ;[1 1 1] camera controls
  (if (`self.InFirstPersonView`)
    (`TurretComponent.ManualAim` (`self.TurretComponent`) AxisValue (stale `InputAxis|AimAzimuth` AxisValue) :!label _label)
    (else
      (`SceneComponent.K2_AddLocalRotation` (`self.SpringArm`) (`KismetMathLibrary.MakeRotator` 0.0 AxisValue) false false))))

(event `InputAction|mouseclick`
  (params (Key :type "Key Structure"))
  ;[1 1 1] handle mouse click
  (:`Pressed`
    (`self.HandleLeftMouseClick`)))

(event `InputAxis|AimAzimuth`
  (params (AxisValue :type "Float (single-precision)"))
  ;[1 1 1] camera controls
  (if (`self.InFirstPersonView`)
    (goto _label)
    (else
      (`SceneComponent.K2_AddLocalRotation` (`self.azimuth_aim_rotation`) (`KismetMathLibrary.MakeRotator` 0.0 0.0 AxisValue) false false))))

(event `InputAxis|zoom`
  (params (AxisValue :type "Float (single-precision)"))
  ;[1 1 1] camera controls
  (if (not (`self.InFirstPersonView`))
    (`SceneComponent.K2_AddLocalOffset` (`self.3rdPersonCamera`) (`KismetMathLibrary.MakeVector` (* AxisValue 30.0)) false false)))

(event `self.ReceiveBeginPlay`
  (bind _aswheel (cast `wheel` (`ChildActorComponent.ChildActor` (`self.ChildActor`))))
  (bind _aswheel_2 (cast `wheel` (`ChildActorComponent.ChildActor` (`self.ChildActor1`))))
  (bind _aswheel_3 (cast `wheel` (`ChildActorComponent.ChildActor` (`self.ChildActor2`))))
  (bind _aswheel_4 (cast `wheel` (`ChildActorComponent.ChildActor` (`self.ChildActor3`))))
  (bind _asfirst_person_camera (cast `/Game/experiments/TankVehicle/FirstPersonCamera` (`ChildActorComponent.ChildActor` (`self.FirstPersonCameraActor`))))
  (`self.FindComponents` (`self.Sphere`) (`self.Cylinder`) _aswheel_2 _aswheel _aswheel_3 _aswheel_4 _asfirst_person_camera)
  (`UA2navcomponent_ground_vehicle.FindActor` (`self.NavigationComponent`) self))

(event `self.SetWidgetTeam`
  (bind _asworld_team_icon_display_bp (cast `/Game/experiments/WorldTeamIconDisplayBP` (`ChildActorComponent.ChildActor` (`self.TeamIcon`))))
  (bind _returnvalue (`self.GetTeam`))
  (`/Game/experiments/WorldTeamIconDisplayBP.SetWidgetTeam` _asworld_team_icon_display_bp _returnvalue)
  (`/Game/experiments/AddToHUD.AddToHudF` (`self.AddToHUD`)))

(fn `UserConstructionScript`)
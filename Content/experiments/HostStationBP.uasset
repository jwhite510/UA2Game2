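; HostStationBP is a player-controllable station with an orbit camera, turret parts and a team icon.
; Mouse clicks go to HandleLeftMouseClick, while axis inputs pitch the spring arm, yaw the azimuth component and zoom by offsetting the camera.
; SetWidgetTeam passes the station's team to its child-actor icon display, then adds it to the HUD.
; The construction script sets the ground-arrow reference and registers turret base and barrel through FindComponents.
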(event `self.ReceiveBeginPlay`)

(event `InputAction|mouseclick`
  (params (Key :type "Key Structure"))
  ;[1 1 1] handle mouse click
  (:`Pressed`
    (`self.HandleLeftMouseClick`)))

(event `InputAxis|AimElevation`
  (params (AxisValue :type "Float (single-precision)"))
  ;[1 1 1] camera controls
  (`SceneComponent.K2_AddLocalRotation` (`self.SpringArm`) (`KismetMathLibrary.MakeRotator` 0.0 AxisValue) false false))

(event `InputAxis|AimAzimuth`
  (params (AxisValue :type "Float (single-precision)"))
  ;[1 1 1] camera controls
  (`SceneComponent.K2_AddLocalRotation` (`self.Azim`) (`KismetMathLibrary.MakeRotator` 0.0 0.0 AxisValue) false false))

(event `InputAxis|zoom`
  (params (AxisValue :type "Float (single-precision)"))
  ;[1 1 1] camera controls
  (`SceneComponent.K2_AddLocalOffset` (`self.Camera`) (`KismetMathLibrary.MakeVector` (* AxisValue 30.0)) false false))

(event `self.SetWidgetTeam`
  (bind _asworld_team_icon_display_bp (cast `/Game/experiments/WorldTeamIconDisplayBP` (`ChildActorComponent.ChildActor` (`self.TeamIcon`))))
  (bind _returnvalue (`self.GetTeam`))
  (`/Game/experiments/WorldTeamIconDisplayBP.SetWidgetTeam` _asworld_team_icon_display_bp _returnvalue)
  (`/Game/experiments/AddToHUD.AddToHudF` (`self.AddToHUD`)))

(fn `UserConstructionScript`
  (set `self.ArrowToGround` (`self.ArrowToGroundBP`))
  (`self.FindComponents` (`self.TurretBase`) (`self.TurretBarrel`)))